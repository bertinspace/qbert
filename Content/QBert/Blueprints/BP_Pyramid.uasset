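; Q*bert level actor that builds a stepped pyramid of BP_Tile actors at BeginPlay, sized by the player's stats level.
; Each layer is a shrinking square ring placed relative to the actor, with four NavLinkProxy_Enemy links per tile for enemy movement.
; Black cats and Sams spawn above random tiles, their counts scaling with level.
; Tick polls the tiles and, once all are coloured, increments the level and reloads the Game map.
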(event `self.ReceiveBeginPlay`
  (`self.Create level`))

(event `Create level`
  (bind _tile_size (`self.Tile Size`))
  (bind _edge_width (`self.Edge Width`))
  (bind _asbp_third_person_character (cast `/Game/ThirdPerson/Blueprints/BP_ThirdPersonCharacter` (`GameplayStatics.GetPlayerCharacter` 0)))
  (bind _level (`/Game/ThirdPerson/Blueprints/BPC_QbertStats.Level` (`/Game/ThirdPerson/Blueprints/BP_ThirdPersonCharacter.BPC_QbertStats` _asbp_third_person_character)))
  (set `self.Levels` (+ _level 5))
  (set `self.Kitties` (+ _level 1))
  (set `self.Sams` _level)
  (for _index (range (+ (`self.Levels`) 1))
    (bind _output_get (set `self.Width` (- (`self.MaxWidth`) (* _index 2))))
    (bind _output_get_2 (set `self.Edge Width` (/ _output_get 2)))
    (bind _returnvalue (* _output_get_2 -1))
    (for _index_2 (range _returnvalue (+ _output_get_2 1))
      (for _index_3 (range _returnvalue (+ _output_get_2 1))
        (if (or (== (`KismetMathLibrary.Abs_Int` _index_3) _edge_width) (== (`KismetMathLibrary.Abs_Int` _index_2) _edge_width))
          (bind _returnvalue_2 (`KismetMathLibrary.MakeVector` (* _index_3 _tile_size) (* _index_2 _tile_size) (* _index (`self.Tile Size`))))
          (bind _returnvalue_3 (`self.Make Local Transform` _returnvalue_2))
          (bind _returnvalue_4 (`|SpawnActorFromClass` "/Game/QBert/Blueprints/BP_Tile.BP_Tile_C" _returnvalue_3 "Undefined" "MultiplyWithRoot" null null))
          (`KismetArrayLibrary.Array_Add` (`self.Tiles`) _returnvalue_4)
          (bind _returnvalue_5 (`self.Make Local Transform` (+ _returnvalue_2 (-200.0 -10.0 20.0))))
          (`|SpawnActorFromClass` "/Game/NavLinkProxy_Enemy.NavLinkProxy_Enemy_C" _returnvalue_5 "Undefined" "MultiplyWithRoot" null null)
          (bind _returnvalue_6 (`self.Make Local Transform` (+ _returnvalue_2 (200.0 -10.0 20.0)) (struct :`Yaw` 180.0)))
          (`|SpawnActorFromClass` "/Game/NavLinkProxy_Enemy.NavLinkProxy_Enemy_C" _returnvalue_6 "Undefined" "MultiplyWithRoot" null null)
          (bind _returnvalue_7 (`self.Make Local Transform` (+ _returnvalue_2 (0.0 200.0 20.0)) (struct :`Yaw` 270.0)))
          (`|SpawnActorFromClass` "/Game/NavLinkProxy_Enemy.NavLinkProxy_Enemy_C" _returnvalue_7 "Undefined" "MultiplyWithRoot" null null)
          (bind _returnvalue_8 (`self.Make Local Transform` (+ _returnvalue_2 (0.0 -200.0 20.0)) (struct :`Yaw` 90.0)))
          (`|SpawnActorFromClass` "/Game/NavLinkProxy_Enemy.NavLinkProxy_Enemy_C" _returnvalue_8 "Undefined" "MultiplyWithRoot" null null)
          (set `self.Last Tile` _returnvalue_2)))))
  (for _ (range 1 (+ (`self.Kitties`) 1))
    (bind _returnvalue_9 (`self.Make Local Transform` (+ (`SceneComponent.K2_GetComponentLocation` (`/Game/QBert/Blueprints/BP_Tile.Body` (`|GetArrayItem` (`self.Tiles`) (`KismetMathLibrary.RandomInteger` (`KismetArrayLibrary.Array_Length` (`self.Tiles`)))))) (0.0 0.0 200.0))))
    (`|SpawnActorFromClass` "/Game/ThirdPerson/Blueprints/BP_Black_Cat.BP_Black_Cat_C" _returnvalue_9 "Undefined" "MultiplyWithRoot" null null))
  (for _ (range 1 (+ (`self.Sams`) 1))
    (bind _returnvalue_10 (`self.Make Local Transform` (+ (`SceneComponent.K2_GetComponentLocation` (`/Game/QBert/Blueprints/BP_Tile.Body` (`|GetArrayItem` (`self.Tiles`) (`KismetMathLibrary.RandomInteger` (`KismetArrayLibrary.Array_Length` (`self.Tiles`)))))) (0.0 0.0 200.0))))
    (`|SpawnActorFromClass` "/Game/ThirdPerson/Blueprints/BP_Sam.BP_Sam_C" _returnvalue_10 "Undefined" "MultiplyWithRoot" null null)))

(event `self.ReceiveTick`
  (params (DeltaSeconds :type "Float (single-precision)"))
  (set `self.ColouredTiles` 0)
  (for _array_element (`self.Tiles`)
    (if (`/Game/QBert/Blueprints/BP_Tile.Coloured` _array_element)
      (set `self.ColouredTiles` (+ (`self.ColouredTiles`) 1))))
  (if (== (`self.ColouredTiles`) (`KismetArrayLibrary.Array_Length` (`self.Tiles`)))
    (`KismetSystemLibrary.PrintString` "Level Up")
    (bind _asbp_third_person_character (cast `/Game/ThirdPerson/Blueprints/BP_ThirdPersonCharacter` (`GameplayStatics.GetPlayerCharacter` 0)))
    (`/Game/ThirdPerson/Blueprints/BPC_QbertStats.IncreaseLevel` (`/Game/ThirdPerson/Blueprints/BP_ThirdPersonCharacter.BPC_QbertStats` _asbp_third_person_character))
    (`GameplayStatics.OpenLevelBySoftObjectPtr` "/Game/QBert/Maps/Game.Game")))

(fn `Make Local Transform`
  (params (Location :type "Vector Structure") (Rotation :type "Rotator Structure") (Scale :type "Vector Structure" :default (1.0 1.0 1.0)))
  (returns (ReturnValue :type "Transform Structure"))
  (return (`KismetMathLibrary.ComposeTransforms` (`self.GetTransform`) (`KismetMathLibrary.MakeTransform` Location Rotation Scale))))

(fn `UserConstructionScript`
  (bind _output_get (set `self.Levels` (+ (/ (`self.MaxWidth`) 2) 1)))
  (set `self.Total Height` (* (- _output_get 1) (`self.Tile Size`))))