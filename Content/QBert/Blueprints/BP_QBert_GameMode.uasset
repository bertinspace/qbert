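; BP_QBert_GameMode is the game mode for a QBert game that handles player lives and respawning.
; On BeginPlay it binds PlayerDead to an OnPlayerDead event.
; When a death fires and lives remain, it decrements PlayerLives, prints the value and restarts the player through the dead character's controller.
; No handling exists for when lives reach zero.
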(event `self.ReceiveBeginPlay`
  (add `self.OnPlayerDead` (delegate `PlayerDead`)))

(event `PlayerDead` :!signature `self.OnPlayerDead`
  (params (Character :type "Character Object Reference"))
  (if (> (`self.PlayerLives`) 0)
    (bind _result (`/Engine/EditorBlueprintResources/StandardMacros.DecrementInt` (`self.PlayerLives`))
      (:`  `
        (`KismetSystemLibrary.PrintString` (`KismetStringLibrary.Conv_IntToString` _result))
        (`self.RestartPlayer` (`Pawn.GetController` Character))))))

(fn `UserConstructionScript`)